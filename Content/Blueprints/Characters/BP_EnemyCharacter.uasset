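; BP_EnemyCharacter is an enemy character with a world-attached health bar widget and hit feedback.
; On BeginPlay it caches the WBP_EnemyHealth widget from its widget component.
; The HealthBarRange overlap shows the bar while the first-person player is inside and hides it when they leave.
; When health changes, it copies the Health component's value into the widget and calls HandleHitFX.
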(event OnComponentBeginOverlap(HealthBarRange)
  (params (OverlappedComponent :type Primitive%20Component%20Object%20Reference) (OtherActor :type Actor%20Object%20Reference) (OtherComp :type Primitive%20Component%20Object%20Reference) (OtherBodyIndex :type Integer) (bFromSweep :type Boolean) (SweepResult :type Hit%20Result%20Structure%20%28by%20ref%29))
  (Utilities|Casting|CastToBP_FirstPersonCharacter OtherActor)
  (Rendering|SetVisibility (Variables|Default|GetHealth%20Bar%20Widget) true false))

(event OnComponentEndOverlap(HealthBarRange)
  (params (OverlappedComponent :type Primitive%20Component%20Object%20Reference) (OtherActor :type Actor%20Object%20Reference) (OtherComp :type Primitive%20Component%20Object%20Reference) (OtherBodyIndex :type Integer))
  (Utilities|Casting|CastToBP_FirstPersonCharacter OtherActor)
  (Rendering|SetVisibility (Variables|Default|GetHealth%20Bar%20Widget) false false))

(event EventBeginPlay
  (bind _aswbp_enemy_health (Utilities|Casting|CastToWBP_EnemyHealth (UserInterface|GetUserWidgetObject (Variables|Default|GetHealth%20Bar%20Widget))))
  (Variables|Default|SetHealth%20Widget%20Reference _aswbp_enemy_health))

(event EventOnHealthChanged
  (Variables|/Game/Blueprints/UI/WBP_EnemyHealth.WBP_EnemyHealth_C|SetHealth (Variables|Default|GetHealth%20Widget%20Reference) (Variables|/Script/VacuumGame.HealthComponent|GetHealth (Variables|Default|GetHealth)))
  (Class|EnemyCharacter|HandleHitFX))

(fn ConstructionScript)